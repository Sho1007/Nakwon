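; BP_Zombie is a zombie character with melee attacks and per-limb dismemberment.
; Loose functions hide arm or leg bones on the mesh and clear that limb's flag.
; Attack, gated by CanAttack, disables movement, then plays a both-hand or single-hand montage matching the remaining arms; with neither arm, no montage plays.
; EndAttack, not called within this Blueprint, re-enables attacking and restores NavWalking movement.
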(event `Attack`
  (if (`self.bCanAttack`)
    (`CharacterMovementComponent.DisableMovement` (`self.CharacterMovement`))
    (if (`self.bLeftArm`)
      (if (`self.bRightArm`)
        (set `self.bCanAttack` false)
        (`self.PlayAnimMontage` "/Game/Resources/Animation/BSP_ZombieAnims/Animations/Standing/Attack/AS_NAAT_Zombie_Attack_BH_Stand_Montage.AS_NAAT_Zombie_Attack_BH_Stand_Montage")
        (else
          (set `self.bCanAttack` false)
          (`self.PlayAnimMontage` "/Game/Resources/Animation/BSP_ZombieAnims/Animations/Standing/Attack/AS_NAAT_Zombie_Attack_LH_Stand_Montage.AS_NAAT_Zombie_Attack_LH_Stand_Montage")))
      (elif (`self.bRightArm`)
        (set `self.bCanAttack` false)
        (`self.PlayAnimMontage` "/Game/Resources/Animation/BSP_ZombieAnims/Animations/Standing/Attack/AS_NAAT_Zombie_Attack_RH_Stand_Montage.AS_NAAT_Zombie_Attack_RH_Stand_Montage")))))

(fn `EndAttack`
  (set `self.bCanAttack` true)
  (`CharacterMovementComponent.SetMovementMode` (`self.CharacterMovement`) "MOVE_NavWalking" 0))

(fn `Loose Left Calf`
  (`SkinnedMeshComponent.HideBoneByName` (`self.Mesh`) "calf_l" "PBO_None")
  (set `self.bLeftLeg` false))

(fn `Loose Left Lower Arm`
  (`SkinnedMeshComponent.HideBoneByName` (`self.Mesh`) "lowerarm_l" "PBO_None")
  (set `self.bLeftArm` false))

(fn `Loose Left Thigh`
  (`SkinnedMeshComponent.HideBoneByName` (`self.Mesh`) "thigh_l" "PBO_None")
  (set `self.bLeftLeg` false))

(fn `Loose Left Upper Arm`
  (`SkinnedMeshComponent.HideBoneByName` (`self.Mesh`) "upperarm_l" "PBO_None")
  (set `self.bLeftArm` false))

(fn `Loose Right Calf`
  (`SkinnedMeshComponent.HideBoneByName` (`self.Mesh`) "calf_r" "PBO_None")
  (set `self.bRightLeg` false))

(fn `Loose Right Lower Arm`
  (`SkinnedMeshComponent.HideBoneByName` (`self.Mesh`) "lowerarm_r" "PBO_None")
  (set `self.bRightArm` false))

(fn `Loose Right Thigh`
  (`SkinnedMeshComponent.HideBoneByName` (`self.Mesh`) "thigh_r" "PBO_None")
  (set `self.bRightLeg` false))

(fn `Loose Right Upper Arm`
  (`SkinnedMeshComponent.HideBoneByName` (`self.Mesh`) "upperarm_r" "PBO_None")
  (set `self.bRightArm` false))

(fn `UserConstructionScript`)