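; AI controller for zombies that runs the BT_Zombie behavior tree on possess and targets the closest perceived player character.
; AI Perception updates add or remove BP_Character actors from a perceived list as they are sensed or lost.
; Each update triggers a distance search over that list, which writes the nearest character to the TargetActor blackboard key and prints debug names.
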(event `self.ReceivePossess`
  (params (PossessedPawn :type "Pawn Object Reference"))
  (`self.RunBehaviorTree` "/Game/Blueprints/AI/BT_Zombie.BT_Zombie"))

(event `self.AIPerception.OnTargetPerceptionUpdated`
  (params (Actor :type "Actor Object Reference") (Stimulus :type "AIStimulus Structure"))
  (bind _asbp_character (cast `/Game/Blueprints/Character/BP_Character` Actor))
  (if (`.bSuccessfullySensed` (break `AIStimulus` Stimulus))
    (`KismetArrayLibrary.Array_Add` (`self.PerceivedActors`) _asbp_character)
    (else
      (`KismetArrayLibrary.Array_RemoveItem` (`self.PerceivedActors`) _asbp_character)))
  (`self.Find Nearest Player`)
  (`KismetSystemLibrary.PrintString` (`KismetSystemLibrary.GetDisplayName` (`BlackboardComponent.GetValueAsObject` (`self.Blackboard`) "TargetActor"))))

(fn `Find Nearest Player`
  (locals (NearestPlayer :type "Actor Object Reference") (NearestDistance :type "Float (double-precision)"))
  (bind _nearestplayer (`local.NearestPlayer`))
  (set `local.NearestDistance` 987654321.0)
  (for _array_element (`self.PerceivedActors`)
    (bind _returnvalue (`self.GetDistanceTo` (`self.K2_GetPawn`) _array_element))
    (if (> (`local.NearestDistance`) _returnvalue)
      (set `local.NearestPlayer` _array_element)
      (set `local.NearestDistance` _returnvalue)))
  (`BlackboardComponent.SetValueAsObject` (`self.Blackboard`) "TargetActor" _nearestplayer)
  (`KismetSystemLibrary.PrintString` (`KismetSystemLibrary.GetDisplayName` _nearestplayer)))

(fn `UserConstructionScript`)