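; Editor utility that turns a static or skeletal mesh into an icon texture and a material instance.
; Loading either mesh type clears the other, and the capture actor's render target is saved as a static texture named after the mesh.
; For static meshes only, a duplicated post-process icon material instance receives that texture.
; Existing assets are replaced by deleting and re-running the event; render target size is set in 64-pixel units.
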(event `LoadSkeletalMesh`
  ;[1 1 1] Load Skeletal Mesh
  (`/Engine/EditorBlueprintResources/StandardMacros.IsValid` (`self.SkeletalMesh`)
    (:`Is Valid`
      (`SkeletalMeshComponent.SetSkeletalMeshAsset` (`self.SkeletalMeshComponent`) (`self.SkeletalMesh`))
      (`StaticMeshComponent.SetStaticMesh` (`self.StaticMeshComponent`) null)
      (set `self.StaticMesh` null))))

(event `LoadStaticMesh`
  ;[1 1 1] Load Static Mesh
  (`/Engine/EditorBlueprintResources/StandardMacros.IsValid` (`self.StaticMesh`)
    (:`Is Valid`
      (`StaticMeshComponent.SetStaticMesh` (`self.StaticMeshComponent`) (`self.StaticMesh`))
      (`SkeletalMeshComponent.SetSkeletalMeshAsset` (`self.SkeletalMeshComponent`) null)
      (set `self.SkeletalMesh` null))))

(event `CreateItemIcon`
  (bind _capturecomponent2d (`SceneCapture2D.CaptureComponent2D` (`self.CaptureActor`)))
  ;[1 1 1] Create RenderTarget
  (`/Engine/EditorBlueprintResources/StandardMacros.IsValid` (`self.StaticMesh`)
    (:`Is Valid`
      (set `self.RTIAssetPath` (`KismetStringLibrary.Concat_StrStr` "/Game/Resources/Texture/Icon/" (`KismetStringLibrary.Concat_StrStr` "RTI_" (`KismetSystemLibrary.GetDisplayName` (`self.StaticMesh`))))))
    (:`Is Not Valid`
      (`/Engine/EditorBlueprintResources/StandardMacros.IsValid` (`self.SkeletalMesh`)
        (:`Is Valid`
          (set `self.RTIAssetPath` (`KismetStringLibrary.Concat_StrStr` "/Game/Resources/Texture/Icon/" (`KismetStringLibrary.Concat_StrStr` "RTI_" (`KismetSystemLibrary.GetDisplayName` (`self.SkeletalMesh`)))))))))
  (`SceneCaptureComponent2D.CaptureScene` _capturecomponent2d)
  (bind _returnvalue (`EditorAssetLibrary.DoesAssetExist` (`self.RTIAssetPath`)))
  (if _returnvalue
    (`EditorAssetLibrary.DeleteAsset` (`self.RTIAssetPath`))
    (`self.CreateItemIcon`)
    (else
      (bind _returnvalue_2 (`KismetRenderingLibrary.RenderTargetCreateStaticTexture2DEditorOnly` (`SceneCaptureComponent2D.TextureTarget` _capturecomponent2d) (`self.RTIAssetPath`) "TC_EditorIcon"))
      (bind _output_get (set `self.GeneratedTextureTarget` _returnvalue_2))
      (`EditorAssetLibrary.SaveLoadedAsset` _output_get))))

(event `SetSize`
  ;[1 1 1] Set Size
  (`KismetRenderingLibrary.ResizeRenderTarget2D` (`self.RTTOrigin`) (* (`self.Width`) 64) (* (`self.Height`) 64)))

(event `CreateMaterialInstance`
  (`/Engine/EditorBlueprintResources/StandardMacros.IsValid` (`self.StaticMesh`)
    (:`Is Valid`
      (`|ExecutionSequence`
        (:`then_0`
          (bind _output_get (set `self.MIAssetName` (`KismetStringLibrary.Concat_StrStr` "MI_" (`KismetSystemLibrary.GetDisplayName` (`self.StaticMesh`)))))
          (set `self.MIAssetPath` (`KismetStringLibrary.Concat_StrStr` "/Game/Resources/Material/Icon/" _output_get)))
        (:`then_1`
          (bind _returnvalue (`EditorAssetLibrary.DoesAssetExist` (`self.MIAssetPath`)))
          (if _returnvalue
            (`EditorAssetLibrary.DeleteAsset` (`self.MIAssetPath`))
            (`self.CreateMaterialInstance`)
            (else
              (bind _returnvalue_2 (`AssetToolsHelpers.GetAssetTools`))
              (bind _returnvalue_3 (`AssetTools.DuplicateAsset` _returnvalue_2 (`self.MIAssetName`) "/Game/Resources/Material/Icon/" "/Game/Resources/Material/MI_PostProcessIcon.MI_PostProcessIcon"))
              (set `self.GeneratedMaterialInstance` _returnvalue_3))))
        (:`then_2`
          (bind _asmaterial_instance (cast `MaterialInstance` (`self.GeneratedMaterialInstance`)))
          (bind _asmaterial_instance_constant (cast `MaterialInstanceConstant` _asmaterial_instance))
          (`MaterialEditingLibrary.SetMaterialInstanceTextureParameterValue` _asmaterial_instance_constant "FinalColorTexture" (`self.GeneratedTextureTarget`))
          (`EditorAssetLibrary.SaveLoadedAsset` (`self.GeneratedMaterialInstance`)))))))

(fn `UserConstructionScript`)